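; Player character Blueprint with basic movement, look, crouching and a toggleable wall-cover system.
; Overlapping a CoverObject enables cover, and a trace toward it supplies the wall normal for a movement plane constraint, with controller yaw rotation disabled.
; While covered, left and right edge traces block movement past the wall's ends, and a center trace updates the normal along the surface.
; Tick ramps CrouchSpeed up or down with crouch state.
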(event `InputAction|Cover`
  (params (Key :type "Key Structure"))
  ;[1 1 1] Covering
  (:`Pressed`
    (if (`self.isCovered`)
      (`self.EndCover`)
      (elif (`self.isAbleToCover`)
        (bind _normal (`self.WallTrace` (`self.CastedObject`)))
        (`self.StartCover` _normal)))))

(event `self.ReceiveActorBeginOverlap`
  (params (OtherActor :type "Actor Object Reference"))
  ;[1 1 1] Covering
  (bind _ascover_object (cast `/Game/World/Objects/CoverObject` OtherActor))
  (set `self.CastedObject` _ascover_object)
  (set `self.isAbleToCover` true))

(event `self.ReceiveActorEndOverlap`
  (params (OtherActor :type "Actor Object Reference"))
  ;[1 1 1] Covering
  (cast `/Game/World/Objects/CoverObject` OtherActor)
  (set `self.isAbleToCover` false))

(event `InputAxis|MoveForward`
  (params (AxisValue :type "Float (single-precision)"))
  ;[1 1 1] Basic Movement
  (bind _output_get (set `self.DirectionY` AxisValue))
  (`self.AddMovementInput` (`KismetMathLibrary.GetForwardVector` (`KismetMathLibrary.MakeRotator` 0.0 0.0 (.yaw (`self.GetControlRotation`)))) _output_get))

(event `InputAxis|MoveRight`
  (params (AxisValue :type "Float (single-precision)"))
  ;[1 1 1] Basic Movement
  (bind _output_get (set `self.DirectionX` AxisValue))
  (if (`self.isCovered`)
    (`self.CoverTrace`)
    (if (== (`self.GetInputAxisValue`) 0.0)
      (`self.AddMovementInput` (* (`MovementComponent.PlaneConstraintNormal` (`self.CharacterMovement`)) 1.0)))
    (else
      (`self.AddMovementInput` (`KismetMathLibrary.GetRightVector` (`KismetMathLibrary.MakeRotator` 0.0 0.0 (.yaw (`self.GetControlRotation`)))) _output_get))))

(event `InputAxis|Turn`
  (params (AxisValue :type "Float (single-precision)"))
  ;[1 1 1] Basic Movement
  (`self.AddControllerYawInput` AxisValue))

(event `InputAxis|LookUp`
  (params (AxisValue :type "Float (single-precision)"))
  ;[1 1 1] Basic Movement
  (`self.AddControllerPitchInput` AxisValue))

(event `InputAction|Crouch`
  (params (Key :type "Key Structure"))
  ;[1 1 1] Crouching
  (:`Pressed`
    (`self.Crouch`))
  (:`Released`
    (`self.UnCrouch`)))

(event `self.ReceiveTick`
  (params (DeltaSeconds :type "Float (single-precision)"))
  (bind _crouchratio (`self.CrouchRatio`))
  (bind _crouchspeed (`self.CrouchSpeed`))
  ;[1 1 1] Crouching
  (if (`NavMovementComponent.IsCrouching` (`self.CharacterMovement`))
    (if (<= _crouchspeed (`self.MaxCrouchSpeed`))
      (set `self.CrouchSpeed` (+ _crouchspeed _crouchratio)))
    (elif (>= _crouchspeed (`self.MinCrouchSpeed`))
      (set `self.CrouchSpeed` (- _crouchspeed _crouchratio)))))

(fn `CoverTrace`
  (locals (LeftHit :type Boolean :default false) (RightHit :type Boolean :default false))
  (bind _returnvalue (`self.K2_GetActorLocation`))
  (bind (_returnvalue_roll _returnvalue_pitch _returnvalue_yaw) (`KismetMathLibrary.BreakRotator` (`self.GetControlRotation`)))
  (bind _returnvalue_2 (`self.GetInputAxisValue`))
  (bind _returnvalue_3 (`KismetMathLibrary.SignOfFloat` _returnvalue_2))
  (bind _planeconstraintnormal (`MovementComponent.PlaneConstraintNormal` (`self.CharacterMovement`)))
  (bind _returnvalue_4 (* (`MovementComponent.PlaneConstraintNormal` (`self.CharacterMovement`)) -1.0))
  (bind _returnvalue_5 (`KismetMathLibrary.GetRightVector` (`KismetMathLibrary.MakeRotator` 0.0 0.0 _returnvalue_yaw)))
  (bind _returnvalue_6 (+ (`self.K2_GetActorLocation`) (* (`KismetMathLibrary.GetRightVector` (`KismetMathLibrary.MakeRotFromX` _planeconstraintnormal)) 30.0)))
  (bind _returnvalue_7 (+ (`self.K2_GetActorLocation`) (* (`KismetMathLibrary.GetRightVector` (`KismetMathLibrary.MakeRotFromX` _returnvalue_4)) 30.0)))
  (`|ExecutionSequence`
    (:`then_0`
      (bind (_outhit _returnvalue_8) (`KismetSystemLibrary.LineTraceSingle` _returnvalue_7 (+ _returnvalue_7 (* _returnvalue_4 200.0)) "TraceTypeQuery3"))
      (set `local.RightHit` _returnvalue_8))
    (:`then_1`
      (bind (_outhit_2 _returnvalue_9) (`KismetSystemLibrary.LineTraceSingle` _returnvalue_6 (+ _returnvalue_6 (* (* _planeconstraintnormal -1.0) 200.0)) "TraceTypeQuery3"))
      (set `local.LeftHit` _returnvalue_9))
    (:`then_2`
      (if (and (`local.RightHit`) (`local.LeftHit`))
        (if (!= (`self.GetInputAxisValue`) 0.0)
          (bind (_outhit_3 _returnvalue_10) (`KismetSystemLibrary.LineTraceSingle` _returnvalue (+ _returnvalue (* (* (`MovementComponent.PlaneConstraintNormal` (`self.CharacterMovement`)) -1.0) 200.0)) "TraceTypeQuery3"))
          (if _returnvalue_10
            (`MovementComponent.SetPlaneConstraintNormal` (`self.CharacterMovement`) (`.Normal` (`GameplayStatics.BreakHitResult` _outhit_3)))
            (`self.AddMovementInput` _returnvalue_5 (`self.GetInputAxisValue`))))
        (else
          (`self.AddMovementInput` _returnvalue_5 (`KismetMathLibrary.SelectFloat` _returnvalue_2 0.0 (and (!= _returnvalue_3 0.0) (select `bool` (== _returnvalue_3 1.0) :`false` (`local.LeftHit`) :`true` (`local.RightHit`))))))))))

(fn `CoverTrigger`)

(fn `EndCover`
  (`MovementComponent.SetPlaneConstraintEnabled` (`self.CharacterMovement`) false)
  (set `self.bUseControllerRotationYaw` true)
  (set `self.isCovered` false))

(fn `StartCover`
  (params (PlaneNormal :type "Vector Structure"))
  (bind _charactermovement (`self.CharacterMovement`))
  (`MovementComponent.SetPlaneConstraintEnabled` _charactermovement true)
  (`MovementComponent.SetPlaneConstraintNormal` _charactermovement PlaneNormal)
  (set `self.bUseControllerRotationYaw` false)
  (set `self.isCovered` true))

(fn `UserConstructionScript`)

(fn `WallTrace`
  (params (Target :type "Actor Object Reference"))
  (returns (Normal :type "Vector Structure"))
  (locals (ObjectTypes :type "Array of EObjectTypeQuery Enum"))
  (bind (_outhit _returnvalue) (`KismetSystemLibrary.LineTraceSingle` (`self.K2_GetActorLocation`) (`self.K2_GetActorLocation` Target) "TraceTypeQuery3"))
  (if _returnvalue
    (return (`.Normal` (`GameplayStatics.BreakHitResult` _outhit)))
    (else
      (`KismetSystemLibrary.PrintString` "Failed"))))